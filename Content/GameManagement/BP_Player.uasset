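; BP_Player is one civilization in a turn-based card game, either the human or a planet-mesh bot opponent.
; BeginPlay gives the human a card-hand HUD and each bot a screen-projected stats widget.
; On RunTurn, bots evoke a random hand card or, with cards in play, activate one, while humans await ability activation, then GameManager advances.
; Players without cards are announced extinct, and a dead human loads GameOver.
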(event Custom|RefreshCardsInHand
  (bind _selfwidget (Variables|Default|GetSelfWidget))
  ;[0 0.7321 1] When the Number of Cards in Hand Changes, tell the Card Stats Widget to Update the Info
  (if (Variables|Default|GetIsBot)
    (Variables|/Script/UMG.TextBlock|SetText (Variables|/Game/UI/EnemyWidget.EnemyWidget_C|GetCardsInHandText _selfwidget) (Utilities|Text|ToText(Integer) (Utilities|Array|Length (Variables|Default|GetCardsInHand))))
    (CallFunction|RelocateUI _selfwidget)))

(event Custom|Run%20Turn
  (bind _staticmeshcomp (Variables|Default|GetStaticMeshComp))
  (bind _returnvalue (Transformation|GetWorldLocation _staticmeshcomp))
  (if (CallFunction|IsPlayerAlive)
    (CallFunction|IndicatorText (Utilities|Text|ToText(String) (Utilities|String|Append (Variables|Default|GetCivilizationName) "'s turn")))
    ;[0 0.546 1] When asked to run a turn, choose a random card and tell the game manager to spawn one, before moving to the next turn.
    (if (Variables|Default|GetIsBot)
      (bind (_chosen_turn_card _turntype _chosen_physical) (CallFunction|ChooseTurnAction))
      (switch Utilities|FlowControl|Switch|SwitchonTurnType _turntype
        (:NewEnumerator1
          (bind _output_get (Variables|Default|SetChosen%20Turn%20Action _chosen_turn_card))
          (CallFunction|EvokeCard _output_get (Math|Vector|MakeVector (+ (.x _returnvalue) 1e+02) (.y _returnvalue) (.z _returnvalue)) self)
          (Utilities|Array|RemoveItem (Variables|Default|GetCardsInHand) (Variables|Default|GetChosen%20Turn%20Action))
          (Default|NextTurn (Variables|Default|GetGameManager) (Variables|Default|GetTurn%20Index)))
        (:NewEnumerator2
          (Variables|/Game/UI/CardUI/WCardPhysical.WCardPhysical_C|SetActivated _chosen_physical true)
          (Default|NextTurn (Variables|Default|GetGameManager) (Variables|Default|GetTurn%20Index))))
      (else
        (CallFunction|RunPlayerTurn)))
    (else
      (Utilities|FlowControl|Sequence
        (:then_0
          ;[1 1 1] If this player is dead, state that they are extinct, once.
          (Utilities|FlowControl|DoOnce false
            (:Completed
              (CallFunction|IndicatorText (Utilities|Text|ToText(String) (Utilities|String|Append (Variables|Default|GetCivilizationName) " is extinct.")))
              (Math|Integer|IncrementInt (Variables|/Game/GameManagement/GameManager.GameManager_C|GetDeadPlayerCount (CallFunction|GetGameManager))))))
        (:then_1
          (Default|NextTurn (Variables|Default|GetGameManager)))
        (:then_2
          ;[1 0.3375 0] If the Human Player is Dead, Go to Death Screen
          (if (not (Variables|Default|GetIsBot))
            (Class|LevelStreamingDynamic|LoadLevelInstancebySoftObjectPtr "/Game/CosmeticLevels/GameOver.GameOver" "0, 0, 0" "0, 0, 0" "" 0 false)))))))

(event Custom|Construct%20Cosmetics
  (params (Chosen%20Planet :type Planet%20Meshes%20Structure))
  ;[1 0 0.1071] This creates the Planet Object if this Player is an Opponent
  (Components|StaticMesh|SetStaticMesh (Variables|Default|GetStaticMeshComp) (Utilities|Struct|BreakPlanetMeshes Chosen%20Planet))
  (Transformation|SetWorldScale3D (Variables|Default|GetStaticMeshComp) "4.000000,4.000000,4.000000"))

(event Custom|Run%20Player%20Turn
  (Variables|Default|SetIs%20Your%20Turn true))

(event Custom|CheckActivateAbility
  (params (Card%20Activated :type W%20Card%20Physical%20Object%20Reference))
  ;[1 1 1] Allow the Activation of a Card by Player, only if owned by player, on the player turn, and only by a player.
  (if (Math|Boolean|ANDBoolean (Variables|Default|GetIs%20Your%20Turn) (Utilities|Array|ContainsItem (Variables|Default|GetPlayed%20Cards) Card%20Activated) (not (Variables|Default|GetIsBot)))
    (Variables|/Game/UI/CardUI/WCardPhysical.WCardPhysical_C|SetActivated Card%20Activated true)
    (Variables|Default|SetIs%20Your%20Turn false)
    (Default|NextTurn (CallFunction|GetGameManager) (Variables|Default|GetTurn%20Index))))

(event EventBeginPlay
  (Variables|Default|SetGameManager (CallFunction|GetGameManager))
  ;[1 0.1121 0.572] At the start of the game, look at the Player and set the game manager variable
  (if (Variables|Default|GetIsBot)
    (Transformation|SetActorRotation (Math|Rotator|FindLookatRotation (Transformation|GetWorldLocation (Variables|Default|GetDefaultSceneRoot)) (Transformation|GetActorLocation (Game|Player|GetPlayerPawn 0))))
    ;[0 0.5781 0.08951] Create the Widget on the Player Screen that shows this Opponent's Stats, and then add it to the viewport in the proper location.
    (bind _output_get (Variables|Default|SetCivilizationName (Utilities|String|Append "Civilization " (Utilities|String|ToString(Integer) (Math|Random|RandomIntegerinRange 1984 42069)))))
    (bind _returnvalue (UserInterface|CreateWidget "/Game/UI/EnemyWidget.EnemyWidget_C" (Game|GetPlayerController 0) "" (Utilities|Text|ToText(String) _output_get) 0))
    (bind _output_get_2 (Variables|Default|SetSelfWidget _returnvalue))
    (Variables|/Script/UMG.TextBlock|SetText (Variables|/Game/UI/EnemyWidget.EnemyWidget_C|GetOpponentText _output_get_2) (Utilities|Text|ToText(String) _output_get))
    (UserInterface|Viewport|AddtoViewport _output_get_2 1)
    (CallFunction|RelocateUI (Variables|Default|GetSelfWidget))
    (else
      (bind _returnvalue_2 (UserInterface|CreateWidget "/Game/UI/CardUI/w_DeveloperHUD.w_DeveloperHUD_C" (Game|GetPlayerController 0)))
      (Variables|Default|SetPlayer%20Widget _returnvalue_2)
      (Variables|/Game/UI/CardUI/wCardZone.wCardZone_C|SetOwningPlayer (Variables|/Game/UI/CardUI/w_DeveloperHUD.w_DeveloperHUD_C|GetwCardHand _returnvalue_2) self)
      (UserInterface|Viewport|AddtoViewport _returnvalue_2 0))))

(fn ConstructionScript)

(fn ChooseTurnAction
  (if (<= (Utilities|Array|Length (Variables|Default|GetPlayed%20Cards)) 0)
    (return (.OutItem (Utilities|Array|Random (Variables|Default|GetCardsInHand))) "NewEnumerator1" 0)
    (else
      (return 0 "NewEnumerator2" (.OutItem (Utilities|Array|Random (Variables|Default|GetPlayed%20Cards)))))))

(fn RelocateUI
  (params (NewParam :type User%20Widget%20Object%20Reference))
  (Class|UserWidget|SetPositioninViewport NewParam (.ScreenLocation (Class|PlayerController|ProjectWorldLocationtoScreen (Game|GetPlayerController 0) (Transformation|GetWorldLocation (Variables|Default|GetDefaultSceneRoot)) false)) true)
  (return))

(fn SelectX
  (params (Zone%20to%20Select%20From :type ZoneType%20Enum :default "NewEnumerator0") (Selection%20Count :type Integer))
  (bind _cardsinhand (Variables|Default|GetCardsInHand))
  (bind _played_cards (Variables|Default|GetPlayed%20Cards))
  (bind _output (Utilities|Array|Get(acopy) _played_cards))
  (bind _output_2 (Utilities|Array|Get(acopy) _cardsinhand))
  (switch Utilities|FlowControl|Switch|SwitchonZoneType Zone%20to%20Select%20From
    (:NewEnumerator0
      (for _index (range 1 Selection%20Count)
        ;[1 1 1] Find X Random cards in Hand (Will have to be Replaced with logic for restricting to specific types)
        (Utilities|Array|Shuffle _cardsinhand)
        (Utilities|Array|Add (LocalVariables|GetTemp%20Hand%20Selected) _output_2)
        (Utilities|Array|RemoveItem _cardsinhand _output_2)))
    (:NewEnumerator3
      (for _index_2 (range 1 Selection%20Count)
        ;[1 1 1] Find X Random cards in Hand (Will have to be Replaced with logic for restricting to specific types)
        (Utilities|Array|Shuffle _played_cards)
        (Utilities|Array|Add (LocalVariables|GetTemp%20Play%20Selected) _output)
        (Utilities|Array|RemoveItem (Variables|Default|GetPlayed%20Cards) _output))))
  (return (LocalVariables|GetTemp%20Hand%20Selected) (LocalVariables|GetTemp%20Play%20Selected)))

(fn IsPlayerAlive
  (return (or (> (Utilities|Array|Length (Variables|Default|GetCardsInHand)) 0) (> (Utilities|Array|Length (Variables|Default|GetPlayed%20Cards)) 0))))