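; BP_CGInstance, by its name a game instance, manages the game's save file through a BP_SaveGame reference.
; Save requests gather every BPI_Saveable actor, have the save object store their data, then write it to a slot.
; Loading reads the slot if it exists and replaces the reference, while data requests are forwarded to the save object.
; Saving and loading run either async or sync and signal completion afterwards.
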(event Custom|Save%20Game
  (params (Async :type Boolean))
  ;[1 0.1012 0.9668] Save the Game either Asynchronously or Sync depending on Bool
  (if Async
    (|AsyncSaveGametoSlot (Variables|Default|GetSave%20Game%20Reference) (Variables|Default|GetSG_SlotName)
      (:Completed
        (Default|CallGameSaveComplete (Variables|Default|GetSave%20Game%20Reference))))
    (else
      (SaveGame|SaveGametoSlot (Variables|Default|GetSave%20Game%20Reference) (Variables|Default|GetSG_SlotName))
      (Default|CallGameSaveComplete (Variables|Default|GetSave%20Game%20Reference)))))

(event Custom|Create%20Save%20Game
  (bind _returnvalue (SaveGame|CreateSaveGameObject "/Game/GameManagement/Save/BP_SaveGame.BP_SaveGame_C"))
  (Variables|Default|SetSave%20Game%20Reference _returnvalue))

(event Custom|LoadGame
  (params (Async :type Boolean))
  (bind _returnvalue (SaveGame|DoesSaveGameExist (Variables|Default|GetSG_SlotName)))
  (if _returnvalue
    (if Async
      (bind _savegame (|AsyncLoadGamefromSlot (Variables|Default|GetSG_SlotName))
        (:Completed
          (bind _asbp_save_game (Utilities|Casting|CastToBP_SaveGame _savegame))
          (bind _output_get (Variables|Default|SetSave%20Game%20Reference _asbp_save_game))
          (Default|CallGameLoaded _output_get)))
      (else
        (bind _returnvalue_2 (SaveGame|LoadGamefromSlot (Variables|Default|GetSG_SlotName)))
        (bind _asbp_save_game_2 (Utilities|Casting|CastToBP_SaveGame _returnvalue_2))
        (bind _output_get_2 (Variables|Default|SetSave%20Game%20Reference _asbp_save_game_2))
        (Default|CallGameLoaded _output_get_2)))))

(event EventRequestSave
  (params (Async :type Boolean))
  ;[1 0 0.7102] For each Saveable Object, Add all Saveable Data to the SaveGame file.
  (bind _outactors (Actor|GetAllActorswithInterface "/Game/GameManagement/Save/BPI_Saveable.BPI_Saveable_C"))
  (Default|SaveAllData (Variables|Default|GetSave%20Game%20Reference) _outactors)
  (CallFunction|SaveGame Async))

(event EventRequestLoad
  (params (Requestor :type Object%20Object%20Reference))
  ;[0 0.1088 1] Pass any data requests to the SaveGame file.
  (Default|LoadDataforRequestor (Variables|Default|GetSave%20Game%20Reference) Requestor))