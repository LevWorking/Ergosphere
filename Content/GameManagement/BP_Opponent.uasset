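; BP_Opponent represents an opponent in a card game, with a generated name and an on-screen widget for its name and hand size.
; On BeginPlay it builds a "Civilization" name with a random number, creates the EnemyWidget and places it once at the actor's projected screen position, without following later movement.
; The RefreshCardsInHand event writes the current CardsInHand count to that widget when called.
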(event Custom|RefreshCardsInHand
  (Variables|/Script/UMG.TextBlock|SetText (Variables|/Game/UI/EnemyWidget.EnemyWidget_C|GetCardsInHandText (Variables|Default|GetSelfWidget)) (Utilities|Text|ToText(Integer) (Utilities|Array|Length (Variables|Default|GetCardsInHand)))))

(event EventBeginPlay
  (bind _output_get (Variables|Default|SetOpponentName (Utilities|String|Append "Civilization " (Utilities|String|ToString(Integer) (Math|Random|RandomIntegerinRange 1984 42069)))))
  (bind _returnvalue (UserInterface|CreateWidget "/Game/UI/EnemyWidget.EnemyWidget_C" (Game|GetPlayerController 0)))
  (bind _output_get_2 (Variables|Default|SetSelfWidget _returnvalue))
  (UserInterface|Viewport|AddtoViewport _output_get_2 1)
  (Variables|/Script/UMG.TextBlock|SetText (Variables|/Game/UI/EnemyWidget.EnemyWidget_C|GetOpponentText _output_get_2) (Utilities|Text|ToText(String) _output_get))
  (Class|UserWidget|SetPositioninViewport (Variables|Default|GetSelfWidget) (.ScreenLocation (Class|PlayerController|ProjectWorldLocationtoScreen (Game|GetPlayerController 0) (Transformation|GetWorldLocation (Variables|Default|GetDefaultSceneRoot)) false)) true))

(event Collision|EventActorBeginOverlap
  (params (OtherActor :type Actor%20Object%20Reference)))

(event EventTick
  (params (DeltaSeconds :type Float%20%28single-precision%29)))

(fn ConstructionScript)